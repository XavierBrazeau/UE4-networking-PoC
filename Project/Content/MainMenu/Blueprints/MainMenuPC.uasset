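; Main menu player controller that creates the main menu widget and adds it to the viewport on BeginPlay.
; Holding V drives push-to-talk voice chat through ToggleSpeaking console commands.
; Debug number keys print test text, including one that calls PlayerPrintString with its index on every ThirdPersonCharacter in the world.
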(event EventBeginPlay
  (bind _returnvalue (UserInterface|CreateWidget "/Game/MainMenu/Blueprints/MainMenuWidgetBP.MainMenuWidgetBP_C" (Game|GetPlayerController 0)))
  (UserInterface|Viewport|AddtoViewport _returnvalue 0))

(event EventTick
  (params (DeltaSeconds :type Float%20%28single-precision%29)))

(event Input|KeyboardEvents|V
  (params (Key :type Key%20Structure :default "None"))
  (bind _returnvalue (Game|GetPlayerController 0))
  (:Pressed
    (Development|ExecuteConsoleCommand "ToggleSpeaking 1" _returnvalue)
    (Development|PrintString "Hello"))
  (:Released
    (Development|ExecuteConsoleCommand "ToggleSpeaking 0" _returnvalue)))

(event Input|KeyboardEvents|1
  (params (Key :type Key%20Structure :default "None"))
  (:Pressed
    (Development|PrintString "Hello")))

(event Input|KeyboardEvents|5
  (params (Key :type Key%20Structure :default "None"))
  (:Pressed
    (bind _outactors (Actor|GetAllActorsOfClass "/Game/ThirdPersonBP/Blueprints/ThirdPersonCharacter.ThirdPersonCharacter_C"))
    (for (_array_element _array_index) _outactors
      (Default|PlayerPrintString _array_element (Utilities|String|ToString(Integer) _array_index)))))

(fn ConstructionScript)